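; BP_Submarine is a keyboard-driven submarine that renders a scan of its surroundings to a screen texture.
; Every tick its Camera captures the scene, then M_ScanScreen is drawn into the RT_ScanResult render target.
; Up and Down presses step the actor along world Y by unequal amounts.
; Left and Right reapply location, pitch and yaw, leaving their intended roll increments unconnected.
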(event Custom|ScanEnvironment
  ;[1 0.8407 0.01328 0.5] Camera Scan
  (Rendering|SceneCapture|CaptureScene (Variables|Default|GetCamera) :!class /Script/Engine.SceneCaptureComponent2D)
  (Rendering|DrawMaterialtoRenderTarget "/Game/Materials/RT_ScanResult.RT_ScanResult" "/Game/Materials/M_ScanScreen.M_ScanScreen"))

(event EventTick
  (params (DeltaSeconds :type Float%20%28single-precision%29))
  (CallFunction|ScanEnvironment))

(event Input|KeyboardEvents|Up
  (params (Key :type Key%20Structure :default "None"))
  (bind _submarine (Variables|Default|GetSubmarine))
  (:Pressed
    (Transformation|SetActorTransform (Math|Transform|MakeTransform (+ (.location (Transformation|GetWorldTransform _submarine)) "0.000000,5.000000,0.000000") (Transformation|GetWorldRotation _submarine) "1.000000,1.000000,1.000000"))))

(event Input|KeyboardEvents|Down
  (params (Key :type Key%20Structure :default "None"))
  (bind _submarine (Variables|Default|GetSubmarine))
  (:Pressed
    (Transformation|SetActorTransform (Math|Transform|MakeTransform (+ (.location (Transformation|GetWorldTransform _submarine)) "0.000000,-1.000000,0.000000") (Transformation|GetWorldRotation _submarine) "1.000000,1.000000,1.000000"))))

(event Input|KeyboardEvents|Left
  (params (Key :type Key%20Structure :default "None"))
  (bind _submarine (Variables|Default|GetSubmarine))
  (bind _returnvalue (Transformation|GetWorldRotation _submarine))
  (:Pressed
    (Transformation|SetActorTransform (Math|Transform|MakeTransform (.location (Transformation|GetWorldTransform _submarine)) (Math|Rotator|MakeRotator 0.0 (.pitch _returnvalue) (.yaw _returnvalue)) "1.000000,1.000000,1.000000"))))

(event Input|KeyboardEvents|Right
  (params (Key :type Key%20Structure :default "None"))
  (bind _submarine (Variables|Default|GetSubmarine))
  (bind _returnvalue (Transformation|GetWorldRotation _submarine))
  (:Pressed
    (Transformation|SetActorTransform (Math|Transform|MakeTransform (.location (Transformation|GetWorldTransform _submarine)) (Math|Rotator|MakeRotator 0.0 (.pitch _returnvalue) (.yaw _returnvalue)) "1.000000,1.000000,1.000000"))))

(fn ConstructionScript)