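; BP_Console is a possessable submarine console that drives a MiniSub and displays its scanner.
; Mouse X yaws the sub, while Mouse Y rolls the Lever, whose angle latches forward or reverse movement applied on Tick until Space zeroes it.
; Tick and the Scan event capture the Scanner scene and draw the scan-screen material to a render target.
; Left click or Disconnect returns possession to the player character.
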(event EventBeginPlay
  (bind _returnvalue (Actor|GetActorOfClass "/Game/Blueprint/BP_Character.BP_Character_C"))
  (Variables|Default|SetPlayerRef _returnvalue))

(event EventDisconnect
  ;[1 0.9138 0] Disconnect
  (bind _asbp_character (Utilities|Casting|CastToBP_Character (Game|GetPlayerCharacter 0)))
  (Pawn|Possess (Game|GetPlayerController 0) _asbp_character))

(event EventScan
  ;[1 0.9138 0] Scan
  (Rendering|SceneCapture|CaptureScene (Variables|Default|GetScanner) :!class /Script/Engine.SceneCaptureComponent2D)
  (Rendering|DrawMaterialtoRenderTarget "/Game/Materials/RT_ScanResult.RT_ScanResult" "/Game/Materials/M_ScanScreen.M_ScanScreen"))

(event EventTick
  (params (DeltaSeconds :type Float%20%28single-precision%29))
  (bind _move_amount (Variables|Default|GetMove%20Amount))
  (Utilities|FlowControl|Sequence
    (:then_0
      (if (== (Variables|Default|GetAccelerationSetting) 1)
        (Transformation|AddWorldOffset (Variables|Default|GetMiniSub) (* (Math|Vector|GetForwardVector (Variables|Default|GetMiniSub)) _move_amount) false false)))
    (:then_1
      (if (== (Variables|Default|GetAccelerationSetting) -1)
        (Transformation|AddWorldOffset (Variables|Default|GetMiniSub) (* (Math|Vector|GetForwardVector (Variables|Default|GetMiniSub)) _move_amount -1.0) false false)))
    (:then_2
      ;[1 0.9138 0] Scan
      (Rendering|SceneCapture|CaptureScene (Variables|Default|GetScanner) :!class /Script/Engine.SceneCaptureComponent2D)
      (Rendering|DrawMaterialtoRenderTarget "/Game/Materials/RT_ScanResult.RT_ScanResult" "/Game/Materials/M_ScanScreen.M_ScanScreen"))))

(event Input|MouseEvents|MouseY
  (params (AxisValue :type Float%20%28single-precision%29))
  (bind _lever (Variables|Default|GetLever))
  (bind _returnvalue (Transformation|GetWorldRotation _lever))
  ;[1 0 0.02609] Acceleration
  (Transformation|SetRelativeRotation (Variables|Default|GetLever) (Math|Rotator|MakeRotator (* AxisValue 3.0) 0.0 -9e+01) false false)
  (if (> (.roll _returnvalue) 2e+01)
    (Variables|Default|SetAccelerationSetting 1)
    (elif (< (.roll _returnvalue) -2e+01)
      (Variables|Default|SetAccelerationSetting -1))))

(event Input|MouseEvents|MouseX
  (params (AxisValue :type Float%20%28single-precision%29))
  (bind _minisub (Variables|Default|GetMiniSub))
  (bind _returnvalue (Transformation|GetWorldRotation _minisub))
  ;[0.7656 0 0.04318] Rotation
  (Transformation|SetWorldRotation (Variables|Default|GetMiniSub) (Math|Rotator|MakeRotator (.roll _returnvalue) (.pitch _returnvalue) (+ (/ AxisValue 8e+01) (.yaw _returnvalue))) false false))

(event Input|KeyboardEvents|SpaceBar
  (params (Key :type Key%20Structure :default "None"))
  ;[1 0 0.02609] Acceleration
  (:Pressed
    (bind _output_get (Variables|Default|SetAccelerationSetting 0))
    (Development|PrintString (Utilities|String|ToString(Integer) _output_get))))

(event Input|MouseEvents|LeftMouseButton
  (params (Key :type Key%20Structure :default "None"))
  (:Pressed
    (Pawn|Possess (Game|GetPlayerController 0) (Variables|Default|GetPlayerRef))))

(fn ConstructionScript)